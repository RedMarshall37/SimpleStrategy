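; Place Blueprint that represents a standing or sitting spot and shows a skeletal mesh at it.
; The Construction Script switches on the PlaceStruct type and adds a skeletal mesh component at the struct's transform, lowered and yawed by fixed offsets.
; It writes the new component back into PlaceStruct; the event graph holds no active logic.
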(event EventBeginPlay)

(event Collision|EventActorBeginOverlap
  (params (OtherActor :type Actor%20Object%20Reference)))

(event EventTick
  (params (DeltaSeconds :type Float%20%28single-precision%29)))

(fn ConstructionScript
  (Variables|Default|SetCoordinates (.transform (Variables|Default|GetPlaceStruct)))
  (switch Utilities|FlowControl|Switch|SwitchonTypeOfPlaceEnum (.type (Variables|Default|GetPlaceStruct))
    (:NewEnumerator0
      (bind _returnvalue (AddComponent|AddSkeletalMeshComponent false (Math|Transform|MakeTransform (Math|Vector|MakeVector (.x (.location (Variables|Default|GetCoordinates))) (.y (.location (Variables|Default|GetCoordinates))) (- (.z (.location (Variables|Default|GetCoordinates))) 8e+01)) (Math|Rotator|MakeRotator (.roll (.rotation (Variables|Default|GetCoordinates))) (.pitch (.rotation (Variables|Default|GetCoordinates))) (- (.yaw (.rotation (Variables|Default|GetCoordinates))) 9e+01)) (.scale (Variables|Default|GetCoordinates)))))
      (Variables|Default|SetPlaceStruct (Utilities|Struct|MakePlaceStructure (.transform (Variables|Default|GetPlaceStruct)) (.type (Variables|Default|GetPlaceStruct)) 0 _returnvalue)))
    (:NewEnumerator1
      (bind _returnvalue_2 (AddComponent|AddSkeletalMeshComponent false (Math|Transform|MakeTransform (Math|Vector|MakeVector (.x (.location (Variables|Default|GetCoordinates))) (.y (.location (Variables|Default|GetCoordinates))) (- (.z (.location (Variables|Default|GetCoordinates))) 8e+01)) (Math|Rotator|MakeRotator (.roll (.rotation (Variables|Default|GetCoordinates))) (.pitch (.rotation (Variables|Default|GetCoordinates))) (- (.yaw (.rotation (Variables|Default|GetCoordinates))) 9e+01)) (.scale (Variables|Default|GetCoordinates)))))
      (Variables|Default|SetPlaceStruct (Utilities|Struct|MakePlaceStructure (.transform (Variables|Default|GetPlaceStruct)) (.type (Variables|Default|GetPlaceStruct)) 0 _returnvalue_2)))))