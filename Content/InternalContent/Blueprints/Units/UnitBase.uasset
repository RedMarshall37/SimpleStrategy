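; Base AI combat unit that moves between Place actors, fires team-tagged bullets and ragdolls when an opposing bullet overlaps it.
; On BeginPlay it copies mesh and offset from the first WeaponBase found, then tracks the left-hand socket each tick.
; Walk and Attack set blackboard targets and the action state, with Walk also transferring Place occupancy.
; Waiting picks stand or sit from the Place type, aligns rotation and ends the task.
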(event OnComponentBeginOverlap(CapsuleComponent)
  (params (OverlappedComponent :type Primitive%20Component%20Object%20Reference) (OtherActor :type Actor%20Object%20Reference) (OtherComp :type Primitive%20Component%20Object%20Reference) (OtherBodyIndex :type Integer) (bFromSweep :type Boolean) (SweepResult :type Hit%20Result%20Structure%20%28by%20ref%29))
  ;[1 1 1] Умираем при попадании пули
  (bind _asbullet_base (Utilities|Casting|CastToBulletBase OtherActor))
  (if (Math|Boolean|NotEqual(Boolean) (Variables|/Game/InternalContent/Blueprints/WeaponsAndBullets/BulletBase.BulletBase_C|GetFromEnemy _asbullet_base) (Variables|Default|GetIsEnemy))
    (Variables|Default|SetIsDeth true)
    (Physics|SetSimulatePhysics (Variables|Character|GetMesh) true)))

(event Custom|Fire
  ;[1 1 1] Стреляем
  (bind _returnvalue (Game|SpawnActorfromClass "/Game/InternalContent/Blueprints/WeaponsAndBullets/BulletBase.BulletBase_C" (Transformation|GetSocketTransform (Variables|Default|GetWeaponMesh) "FirePlace" "RTS_World") "AlwaysSpawn" 0 0))
  (Variables|/Game/InternalContent/Blueprints/WeaponsAndBullets/BulletBase.BulletBase_C|SetFromEnemy _returnvalue (Variables|Default|GetIsEnemy)))

(event EventBeginPlay
  (bind _weaponmesh (Variables|Default|GetWeaponMesh))
  ;[1 1 1] Выдаём оружие боту
  (bind _outactors (Actor|GetAllActorsOfClass "/Game/InternalContent/Blueprints/WeaponsAndBullets/WeaponBase.WeaponBase_C"))
  (Variables|Default|SetWeapon (Utilities|Array|Get(acopy) _outactors))
  (|CallParentFunction)
  (Components|StaticMesh|SetStaticMesh _weaponmesh (Variables|/Game/InternalContent/Blueprints/WeaponsAndBullets/WeaponBase.WeaponBase_C|GetMesh (Variables|Default|GetWeapon)))
  (Transformation|SetRelativeTransform _weaponmesh (Variables|/Game/InternalContent/Blueprints/WeaponsAndBullets/WeaponBase.WeaponBase_C|GetMeshOffset (Variables|Default|GetWeapon)) false false))

(event EventTick
  (params (DeltaSeconds :type Float%20%28single-precision%29))
  ;[1 1 1] Обновляем перменную положения оружия
  (Variables|Default|SetWeaponLocation (.location (Transformation|GetSocketTransform (Variables|Default|GetWeaponMesh) "SocketLeftHand" "RTS_World"))))

(fn ConstructionScript)

(fn Walk
  (params (ThePlaceToGo :type Object%20Object%20Reference))
  (bind _self self)
  (bind _returnvalue (AI|GetBlackboard _self))
  (Utilities|IsValid (Variables|Default|GetCurrentPlace)
    (:Is%20Valid
      (Variables|/Game/InternalContent/Blueprints/Places/Place.Place_C|SetPlaceStruct (Variables|Default|GetCurrentPlace) (Utilities|Struct|MakePlaceStructure (.transform (Variables|/Game/InternalContent/Blueprints/Places/Place.Place_C|GetPlaceStruct (Variables|Default|GetCurrentPlace))) (.type (Variables|/Game/InternalContent/Blueprints/Places/Place.Place_C|GetPlaceStruct (Variables|Default|GetCurrentPlace))) 0 (.model (Variables|/Game/InternalContent/Blueprints/Places/Place.Place_C|GetPlaceStruct (Variables|Default|GetCurrentPlace))))))
    (:Is%20Not%20Valid
      _))
  (bind _asplace (Utilities|Casting|CastToPlace ThePlaceToGo))
  (Variables|Default|SetCurrentPlace _asplace)
  (Variables|/Game/InternalContent/Blueprints/Places/Place.Place_C|SetPlaceStruct _asplace (Utilities|Struct|MakePlaceStructure (.transform (Variables|/Game/InternalContent/Blueprints/Places/Place.Place_C|GetPlaceStruct _asplace)) (.type (Variables|/Game/InternalContent/Blueprints/Places/Place.Place_C|GetPlaceStruct _asplace)) self (.model (Variables|/Game/InternalContent/Blueprints/Places/Place.Place_C|GetPlaceStruct _asplace))))
  (AI|Components|Blackboard|SetValueasObject _returnvalue (Utilities|Name|MakeLiteralName "TargetObject") ThePlaceToGo)
  (AI|Components|Blackboard|SetValueasVector _returnvalue (Utilities|Name|MakeLiteralName "TargetLocation") (Transformation|GetActorLocation _asplace))
  (Variables|Default|SetCurrentAction "NewEnumerator1")
  (Variables|Default|SetIsExecuteTheTask true)
  (bind _asplace_2 (Utilities|Casting|CastToPlace (AI|Components|Blackboard|GetValueasObject (AI|GetBlackboard self) (Utilities|Name|MakeLiteralName "TargetObject")))))

(fn Attack
  (params (TheObjectToAttack :type Object%20Object%20Reference))
  (switch Utilities|FlowControl|Switch|SwitchonCurrentUnitActionEnum (Variables|Default|GetCurrentAction)
    (:NewEnumerator0
      (Variables|Default|SetCurrentAction "NewEnumerator0" :!label _label))
    (:NewEnumerator5
      (Variables|Default|SetCurrentAction "NewEnumerator5" :!label _label_2))
    (:NewEnumerator1
      (goto _label))
    (:NewEnumerator4
      (goto _label))
    (:NewEnumerator6
      (goto _label_2))
    (:NewEnumerator2
      (goto _label))
    (:NewEnumerator7
      (goto _label_2))
    (:NewEnumerator3
      (goto _label))
    (:NewEnumerator8
      (goto _label_2)))
  (AI|Components|Blackboard|SetValueasObject (AI|GetBlackboard self) (Utilities|Name|MakeLiteralName "TargetObject") TheObjectToAttack)
  (Variables|Default|SetIsExecuteTheTask true))

(fn Waiting
  (bind _asplace (Utilities|Casting|CastToPlace (AI|Components|Blackboard|GetValueasObject (AI|GetBlackboard self) (Utilities|Name|MakeLiteralName "TargetObject"))))
  (if (Utilities|Enum|Equal(Enum) (.type (Variables|/Game/InternalContent/Blueprints/Places/Place.Place_C|GetPlaceStruct _asplace)) "NewEnumerator0")
    (Variables|UnitBase_C|SetCurrentAction self "NewEnumerator0")
    (else
      (Variables|UnitBase_C|SetCurrentAction self "NewEnumerator5")))
  (Transformation|SetActorRotation self (Math|Rotator|MakeRotator (.roll (Transformation|GetWorldRotation (.model (Variables|/Game/InternalContent/Blueprints/Places/Place.Place_C|GetPlaceStruct _asplace)))) (.pitch (Transformation|GetWorldRotation (.model (Variables|/Game/InternalContent/Blueprints/Places/Place.Place_C|GetPlaceStruct _asplace)))) (+ (.yaw (Transformation|GetWorldRotation (.model (Variables|/Game/InternalContent/Blueprints/Places/Place.Place_C|GetPlaceStruct _asplace)))) 9e+01)))
  (Variables|Default|SetIsExecuteTheTask false))