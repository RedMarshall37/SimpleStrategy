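; Capture point that allied and enemy units contest, switching between Allies, Enemies and Neutral ownership.
; Box overlaps register units by side; a delay-throttled Tick prunes dead ones, shifts control points by head count and calls CheckOwner to flip owner and blink the decal.
; It also plans defense, choosing quadrants from the attackers' XY bounds and spreading officer positions along those edges, or at the center when officers are too few.
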(event OnComponentBeginOverlap(Box)
  (params (OverlappedComponent :type Primitive%20Component%20Object%20Reference) (OtherActor :type Actor%20Object%20Reference) (OtherComp :type Primitive%20Component%20Object%20Reference) (OtherBodyIndex :type Integer) (bFromSweep :type Boolean) (SweepResult :type Hit%20Result%20Structure%20%28by%20ref%29))
  (bind _asunit_base (Utilities|Casting|CastToUnitBase OtherActor))
  (if (Variables|/Game/InternalContent/Blueprints/Units/UnitBase.UnitBase_C|GetIsEnemy _asunit_base)
    (Math|Integer|IncrementInt (Variables|Default|GetNumberOfEnemyes)
      (:%20%20
        (Utilities|Array|AddUnique (Variables|Default|GetEnemies) _asunit_base)))
    (else
      (Math|Integer|IncrementInt (Variables|Default|GetNumberOfAllies)
        (:%20%20
          (Utilities|Array|AddUnique (Variables|Default|GetAllies) _asunit_base))))))

(event EventTick
  (params (DeltaSeconds :type Float%20%28single-precision%29))
  (Utilities|FlowControl|Delay 0.125)
  (for _array_element (Variables|Default|GetEnemies)
    (if (Variables|/Game/InternalContent/Blueprints/Units/UnitBase.UnitBase_C|GetIsDeth _array_element)
      (Utilities|Array|RemoveItem (Variables|Default|GetEnemies) _array_element)
      (Math|Float|DecrementFloat (Variables|Default|GetEnemyPoints))))
  (for _array_element_2 (Variables|Default|GetAllies)
    (if (Variables|/Game/InternalContent/Blueprints/Units/UnitBase.UnitBase_C|GetIsDeth _array_element_2)
      (Utilities|Array|RemoveItem (Variables|Default|GetAllies) _array_element_2)
      (Math|Float|DecrementFloat (Variables|Default|GetAlliedPoints))))
  (switch Utilities|FlowControl|Switch|SwitchonControlPointEnum (Variables|Default|GetOwnerPoint)
    (:NewEnumerator0
      (CallFunction|CheckOwner (Variables|Default|GetAlliedPoints) (Variables|Default|GetEnemyPoints) "NewEnumerator1" "/Game/InternalContent/Materials/AlliesDecal.AlliesDecal" "/Game/InternalContent/Materials/EnemyDecal.EnemyDecal"))
    (:NewEnumerator1
      (CallFunction|CheckOwner (Variables|Default|GetEnemyPoints) (Variables|Default|GetAlliedPoints) "NewEnumerator0" "/Game/InternalContent/Materials/EnemyDecal.EnemyDecal" "/Game/InternalContent/Materials/AlliesDecal.AlliesDecal"))
    (:NewEnumerator2
      (if (> (Variables|Default|GetNumberOfAllies) (Variables|Default|GetNumberOfEnemyes))
        (CallFunction|CheckOwner (Variables|Default|GetNeutralPoints) (Variables|Default|GetAlliedPoints) "NewEnumerator0" "/Game/InternalContent/Materials/NeutralDecal.NeutralDecal" "/Game/InternalContent/Materials/AlliesDecal.AlliesDecal")
        (else
          (CallFunction|CheckOwner (Variables|Default|GetNeutralPoints) (Variables|Default|GetEnemyPoints) "NewEnumerator1" "/Game/InternalContent/Materials/NeutralDecal.NeutralDecal" "/Game/InternalContent/Materials/EnemyDecal.EnemyDecal")))))
  (if (or (> (Variables|Default|GetNumberOfAllies) 0) (> (Variables|Default|GetNumberOfEnemyes) 0))
    (switch Utilities|FlowControl|Switch|SwitchonControlPointEnum (Variables|Default|GetOwnerPoint)
      (:NewEnumerator0
        (if (> (Variables|Default|GetNumberOfAllies) (Variables|Default|GetNumberOfEnemyes))
          (if (< (Variables|Default|GetAlliedPoints) 1e+02)
            (Math|Float|IncrementFloat (Variables|Default|GetAlliedPoints)))
          (elif (>= (Variables|Default|GetAlliedPoints) 0.0)
            (Math|Float|DecrementFloat (Variables|Default|GetAlliedPoints))
            (else
              (Math|Float|IncrementFloat (Variables|Default|GetEnemyPoints))))))
      (:NewEnumerator1
        (if (> (Variables|Default|GetNumberOfAllies) (Variables|Default|GetNumberOfEnemyes))
          (if (>= (Variables|Default|GetEnemyPoints) 0.0)
            (Math|Float|DecrementFloat (Variables|Default|GetEnemyPoints))
            (else
              (Math|Float|IncrementFloat (Variables|Default|GetAlliedPoints))))
          (elif (< (Variables|Default|GetEnemyPoints) 1e+02)
            (Math|Float|IncrementFloat (Variables|Default|GetEnemyPoints)))))
      (:NewEnumerator2
        (if (>= (Variables|Default|GetNeutralPoints) 0.0)
          (Math|Float|DecrementFloat (Variables|Default|GetNeutralPoints))
          (elif (> (Variables|Default|GetNumberOfAllies) (Variables|Default|GetNumberOfEnemyes))
            (Math|Float|IncrementFloat (Variables|Default|GetAlliedPoints))
            (else
              (Math|Float|IncrementFloat (Variables|Default|GetEnemyPoints)))))))))

(fn ConstructionScript
  (bind _new_scale (Variables|Default|GetNew%20Scale))
  (bind (_x _y _z) (Math|Vector|BreakVector _new_scale))
  (Transformation|SetWorldScale3D (Variables|Default|GetBox) _new_scale)
  (Transformation|SetWorldScale3D (Variables|Default|GetCube) (Math|Vector|MakeVector (* _x 0.65) (* _y 0.65) 0.1))
  (Transformation|SetWorldScale3D (Variables|Default|GetDecal) (Math|Vector|MakeVector (* _x 0.25) (* _y 0.125) 0.01)))

(fn GetSquaretoDefend
  (params (Attackers :type Array%20of%20Unit%20Base%20Object%20References))
  (bind _self self)
  (bind _returnvalue (Transformation|GetActorLocation _self))
  (bind (_maxx _maxy _minx _miny) (CallFunction|MaxandMinXandY Attackers))
  (LocalVariables|SetUnitMaxX _maxx)
  (LocalVariables|SetUnitMaxY _maxy)
  (LocalVariables|SetUnitMinX _minx)
  (LocalVariables|SetUnitMinY _miny)
  (LocalVariables|SetPointX (.x _returnvalue))
  (LocalVariables|SetPointY (.y _returnvalue))
  (CallFunction|CheckSquare (LocalVariables|GetUnitMinX) (LocalVariables|GetUnitMaxY) (LocalVariables|GetPointX) (LocalVariables|GetPointY) false true (Variables|Static|GetTopLeft))
  (CallFunction|CheckSquare (LocalVariables|GetUnitMaxX) (LocalVariables|GetUnitMaxY) (LocalVariables|GetPointX) (LocalVariables|GetPointY) true true (Variables|Static|GetTopRight))
  (CallFunction|CheckSquare (LocalVariables|GetUnitMinX) (LocalVariables|GetUnitMinY) (LocalVariables|GetPointX) (LocalVariables|GetPointY) false false (Variables|Static|GetDownLeft))
  (CallFunction|CheckSquare (LocalVariables|GetUnitMaxX) (LocalVariables|GetUnitMinY) (LocalVariables|GetPointX) (LocalVariables|GetPointY) true false (Variables|Static|GetDownRight))
  (return (Variables|Default|GetSquaresToProtect)))

(fn MaxandMinXandY
  (params (Units :type Array%20of%20Unit%20Base%20Object%20References))
  (for _array_element Units
    (if (LocalVariables|GetFirst)
      (LocalVariables|SetFirst false)
      (LocalVariables|SetMin%20X (.x (Transformation|GetActorLocation _array_element)))
      (LocalVariables|SetMin%20Y (.y (Transformation|GetActorLocation _array_element)))
      (LocalVariables|SetMax%20X (.x (Transformation|GetActorLocation _array_element)))
      (LocalVariables|SetMax%20Y (.y (Transformation|GetActorLocation _array_element)))
      (else
        (LocalVariables|SetMax%20X (Math|Float|Max(Float) (.x (Transformation|GetActorLocation _array_element)) (LocalVariables|GetMax%20X)))
        (LocalVariables|SetMax%20Y (Math|Float|Max(Float) (.y (Transformation|GetActorLocation _array_element)) (LocalVariables|GetMax%20Y)))
        (LocalVariables|SetMin%20X (Math|Float|Min(Float) (.x (Transformation|GetActorLocation _array_element)) (LocalVariables|GetMin%20X)))
        (LocalVariables|SetMin%20Y (Math|Float|Min(Float) (.y (Transformation|GetActorLocation _array_element)) (LocalVariables|GetMin%20Y))))))
  (return (LocalVariables|GetMax%20X) (LocalVariables|GetMax%20Y) (LocalVariables|GetMin%20X) (LocalVariables|GetMin%20Y)))

(fn CheckSquare
  (params (Unit%20X :type Float%20%28single-precision%29) (Unit%20Y :type Float%20%28single-precision%29) (PointX :type Float%20%28single-precision%29) (PointY :type Float%20%28single-precision%29) (MaxX%20%28RightSide%29 :type Boolean) (MaxY%20%28TopSide%29 :type Boolean) (Square%20Name%20 :type Name))
  ;[1 1 1] Записываем переменные, дабы избежать мяса
  (LocalVariables|SetUnitX Unit%20X)
  (LocalVariables|SetUnitY Unit%20Y)
  (LocalVariables|SetPoint%20X PointX)
  (LocalVariables|SetPoint%20Y PointY)
  (LocalVariables|SetMaxX%28RightSide%29 MaxX%20%28RightSide%29)
  (LocalVariables|SetMaxY%28TopSide%29 MaxY%20%28TopSide%29)
  (LocalVariables|SetSquare%20Name Square%20Name%20)
  ;[1 1 1] Нас интересуют кваадраты справа от центра точки?
  (if (LocalVariables|GetMaxX%28RightSide%29)
    ;[1 1 1] Крайний правый враг находится левее центра точки
    (if (> (LocalVariables|GetUnitX) (LocalVariables|GetPoint%20X))
      ;[1 0 0] Y оказался инвертирован
      ;;[1 1 1] Нас интересуют значения впереди от центра точки?
      (if (LocalVariables|GetMaxY%28TopSide%29) :!label _label
        ;;[1 1 1] Самый дальний враг находится впереди от центра точки
        (if (> (LocalVariables|GetUnitY) (LocalVariables|GetPoint%20Y))
          ;[1 1 1] Говорим защищать этот квадрат
          (Utilities|Array|AddUnique (Variables|Default|GetSquaresToProtect) (LocalVariables|GetSquare%20Name) :!label _label_2))
        (else
          ;;[1 1 1] Самый нижний враг находится позади от центра точки
          (if (< (LocalVariables|GetUnitY) (LocalVariables|GetPoint%20Y))
            (goto _label_2)))))
    (else
      ;[1 1 1] Крайний левый враг находится левее центра точки
      (if (< (LocalVariables|GetUnitX) (LocalVariables|GetPoint%20X))
        (goto _label)))))

(fn GetCoordinatesforDefendPerimeter
  (params (Attackers :type Array%20of%20Unit%20Base%20Object%20References) (DefenderOfficers :type Array%20of%20Officer%20Object%20References))
  (bind _returnvalue (Utilities|Array|Length DefenderOfficers))
  (bind _self self)
  (bind _self_2 self)
  (bind _self_3 self)
  (bind _self_4 self)
  (bind _box (Variables|Default|GetBox))
  (bind _returnvalue_2 (Transformation|GetActorLocation _self_2))
  (bind _returnvalue_3 (Transformation|GetActorLocation _self_3))
  (bind _returnvalue_4 (Transformation|GetActorLocation _self))
  (bind _returnvalue_5 (Transformation|GetActorLocation _self_4))
  (bind _returnvalue_6 (Transformation|GetWorldScale _box))
  (bind _squares (CallFunction|GetSquaretoDefend Attackers))
  (if (> (Math|Float|Truncate (/ (Math|Conversions|ToFloat(Integer) _returnvalue) (Math|Conversions|ToFloat(Integer) (Utilities|Array|Length _squares)))) 0)
    (LocalVariables|SetUnitsBySquare (Math|Float|Truncate (/ (Math|Conversions|ToFloat(Integer) _returnvalue) (Math|Conversions|ToFloat(Integer) (Utilities|Array|Length _squares)))))
    (for _array_element _squares
      (LocalVariables|SetOffsetX (/ (* (.x _returnvalue_6) 64.0) 2.0))
      (LocalVariables|SetOffsetY (/ (* (.y _returnvalue_6) 64.0) 2.0))
      (switch name _array_element
        (:TopLeft
          (LocalVariables|SetCurrentCorner (Math|Vector|MakeVector (- (.x _returnvalue_2) (LocalVariables|GetOffsetX)) (+ (.y _returnvalue_2) (LocalVariables|GetOffsetY)) 0.0))
          (bind _returnresults (CallFunction|SetCoordinates (LocalVariables|GetUnitsBySquare) (LocalVariables|GetResults) (LocalVariables|GetCurrentCorner) (LocalVariables|GetOffsetX) (LocalVariables|GetOffsetY) true false))
          (LocalVariables|SetResults _returnresults))
        (:TopRight
          (LocalVariables|SetCurrentCorner (Math|Vector|MakeVector (+ (LocalVariables|GetOffsetX) (.x _returnvalue_5)) (+ (.y _returnvalue_5) (LocalVariables|GetOffsetY)) 0.0))
          (bind _returnresults_2 (CallFunction|SetCoordinates (LocalVariables|GetUnitsBySquare) (LocalVariables|GetResults) (LocalVariables|GetCurrentCorner) (LocalVariables|GetOffsetX) (LocalVariables|GetOffsetY) false false))
          (LocalVariables|SetResults _returnresults_2))
        (:DownLeft
          (LocalVariables|SetCurrentCorner (Math|Vector|MakeVector (- (.x _returnvalue_3) (LocalVariables|GetOffsetX)) (- (.y _returnvalue_3) (LocalVariables|GetOffsetY)) 0.0))
          (bind _returnresults_3 (CallFunction|SetCoordinates (LocalVariables|GetUnitsBySquare) (LocalVariables|GetResults) (LocalVariables|GetCurrentCorner) (LocalVariables|GetOffsetX) (LocalVariables|GetOffsetY) true true))
          (LocalVariables|SetResults _returnresults_3))
        (:DownRight
          (LocalVariables|SetCurrentCorner (Math|Vector|MakeVector (+ (LocalVariables|GetOffsetX) (.x _returnvalue_4)) (- (.y _returnvalue_4) (LocalVariables|GetOffsetY)) 0.0))
          (bind _returnresults_4 (CallFunction|SetCoordinates (LocalVariables|GetUnitsBySquare) (LocalVariables|GetResults) (LocalVariables|GetCurrentCorner) (LocalVariables|GetOffsetX) (LocalVariables|GetOffsetY) false true))
          (LocalVariables|SetResults _returnresults_4))))
    (else
      (for _index (range (- _returnvalue 1) 0)
        (Utilities|Array|Add (LocalVariables|GetResults) (Transformation|GetActorLocation self)))))
  (return (LocalVariables|GetResults)))

(fn SetCoordinates
  (params (UnitsBySquare :type Integer) (Results :type Array%20of%20Vectors) (CurrentCorner :type Vector%20%28by%20ref%29) (OffsetX :type Float%20%28single-precision%29) (OffsetY :type Float%20%28single-precision%29) (X%20increases :type Boolean) (Y%20increases :type Boolean))
  (LocalVariables|SetUnits%20By%20Square UnitsBySquare)
  (LocalVariables|SetResultsLocal Results)
  (LocalVariables|SetCurrent%20Corner CurrentCorner)
  (LocalVariables|SetOffset%20X OffsetX)
  (LocalVariables|SetOffset%20Y OffsetY)
  (LocalVariables|SetXIncreases X%20increases)
  (LocalVariables|SetYIncrease Y%20increases)
  (if (== (Math|Integer|%(Integer) (LocalVariables|GetUnits%20By%20Square) 2) 0)
    (LocalVariables|SetCurrentUnitsBySquare (LocalVariables|GetUnits%20By%20Square))
    (else
      (Utilities|Array|Add (LocalVariables|GetResultsLocal) (LocalVariables|GetCurrent%20Corner))
      (LocalVariables|SetCurrentUnitsBySquare (- (LocalVariables|GetUnits%20By%20Square) 1))))
  (for _index (range 0 (- (/ (LocalVariables|GetCurrentUnitsBySquare) 2) 1))
    (if (LocalVariables|GetXIncreases)
      (LocalVariables|SetCurrentX (+ (.x (LocalVariables|GetCurrent%20Corner)) (* _index (/ (Math|Vector|Distance(Vector) (Math|Vector|MakeVector (.x (LocalVariables|GetCurrent%20Corner)) 0.0 0.0) (Math|Vector|MakeVector (.x (Transformation|GetActorLocation self)) 0.0 0.0)) (Math|Conversions|ToFloat(Integer) (LocalVariables|GetCurrentUnitsBySquare))))))
      (else
        (LocalVariables|SetCurrentX (- (.x (LocalVariables|GetCurrent%20Corner)) 1.0))))
    (if (LocalVariables|GetYIncrease)
      (LocalVariables|SetCurrentY (- (.y (Transformation|GetActorLocation self)) (LocalVariables|GetOffset%20Y)))
      (else
        (LocalVariables|SetCurrentY (+ (.y (Transformation|GetActorLocation self)) (LocalVariables|GetOffset%20Y)))))
    (Utilities|Array|Add (LocalVariables|GetResultsLocal) (Math|Vector|MakeVector (LocalVariables|GetCurrentX) (LocalVariables|GetCurrentY) 0.0)))
  (for _index_2 (range 0 (- (/ (LocalVariables|GetCurrentUnitsBySquare) 2) 1))
    (if (LocalVariables|GetXIncreases)
      (LocalVariables|SetCurrentX (- (.x (Transformation|GetActorLocation self)) (LocalVariables|GetOffset%20X)))
      (else
        (LocalVariables|SetCurrentX (+ (.x (Transformation|GetActorLocation self)) (LocalVariables|GetOffset%20X)))))
    (if (LocalVariables|GetYIncrease)
      (LocalVariables|SetCurrentY (+ (.y (LocalVariables|GetCurrent%20Corner)) (* _index_2 (/ (Math|Vector|Distance(Vector) (Math|Vector|MakeVector 0.0 (.y (LocalVariables|GetCurrent%20Corner)) 0.0) (Math|Vector|MakeVector 0.0 (.y (Transformation|GetActorLocation self)) 0.0)) (Math|Conversions|ToFloat(Integer) (LocalVariables|GetCurrentUnitsBySquare))))))
      (else
        (LocalVariables|SetCurrentY (- (.y (LocalVariables|GetCurrent%20Corner)) (* _index_2 (/ (Math|Vector|Distance(Vector) (Math|Vector|MakeVector 0.0 (.y (LocalVariables|GetCurrent%20Corner)) 0.0) (Math|Vector|MakeVector 0.0 (.y (Transformation|GetActorLocation self)) 0.0)) (Math|Conversions|ToFloat(Integer) (LocalVariables|GetCurrentUnitsBySquare))))))))
    (Utilities|Array|Add (LocalVariables|GetResultsLocal) (Math|Vector|MakeVector (LocalVariables|GetCurrentX) (LocalVariables|GetCurrentY) 0.0)))
  (return (LocalVariables|GetResultsLocal)))

(fn CheckOwner
  (params (Control%20Points :type Float%20%28single-precision%29) (Invaders%20Points :type Float%20%28single-precision%29) (Next%20Owner :type ControlPointEnum%20Enum :default "NewEnumerator0") (Decal%20Material%20Current :type Material%20Interface%20Object%20Reference) (Decal%20Material%20Invaders :type Material%20Interface%20Object%20Reference))
  (LocalVariables|SetControlPoints Control%20Points)
  (LocalVariables|SetInvadersPoints Invaders%20Points)
  (LocalVariables|SetNewOwner Next%20Owner)
  (LocalVariables|SetCurrentDecalMaterial Decal%20Material%20Current)
  (LocalVariables|SetInvadersDecalMaterial Decal%20Material%20Invaders)
  (if (Math|Float|InRange(Float) (LocalVariables|GetControlPoints) 0.0 1e+02 false false)
    (if (Variables|Default|GetFlipFlop)
      (Rendering|Components|Decal|SetDecalMaterial (Variables|Default|GetDecal) (LocalVariables|GetCurrentDecalMaterial))
      (Variables|Default|SetFlipFlop false)
      (else
        (Rendering|Components|Decal|SetDecalMaterial (Variables|Default|GetDecal) "/Game/InternalContent/Materials/NonelDecal.NonelDecal")
        (Variables|Default|SetFlipFlop true)))
    (elif (<= (LocalVariables|GetControlPoints) 0.0)
      (if (>= (LocalVariables|GetInvadersPoints) 1e+02)
        (Variables|Default|SetOwnerPoint (LocalVariables|GetNewOwner))
        (Rendering|Components|Decal|SetDecalMaterial (Variables|Default|GetDecal) (LocalVariables|GetInvadersDecalMaterial))
        (elif (Variables|Default|GetFlipFlop)
          (Rendering|Components|Decal|SetDecalMaterial (Variables|Default|GetDecal) (LocalVariables|GetInvadersDecalMaterial))
          (Variables|Default|SetFlipFlop false)
          (else
            (Rendering|Components|Decal|SetDecalMaterial (Variables|Default|GetDecal) "/Game/InternalContent/Materials/NonelDecal.NonelDecal")
            (Variables|Default|SetFlipFlop true))))
      (elif (>= (LocalVariables|GetControlPoints) 1e+02)
        (Rendering|Components|Decal|SetDecalMaterial (Variables|Default|GetDecal) (LocalVariables|GetCurrentDecalMaterial))))))