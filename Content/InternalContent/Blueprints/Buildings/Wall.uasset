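; Modular building wall that assembles itself from child actors on a 250-unit grid of columns and rows.
; The construction script calls Construct with Width and Height when MastToConstruct is set.
; Intact walls fill every row from column 0 through Width inclusive, while IsDestroyed shortens each higher row into a stepped ruin.
; Separate spawn branches handle the bottom row and, in destroyed walls, each row's end piece.
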(event EventBeginPlay)

(event Collision|EventActorBeginOverlap
  (params (OtherActor :type Actor%20Object%20Reference)))

(event EventTick
  (params (DeltaSeconds :type Float%20%28single-precision%29)))

(fn ConstructionScript
  (if (Variables|Default|GetMastToConstruct)
    (CallFunction|Construct (Variables|Default|GetWidth) (Variables|Default|GetHeight))))

(fn Construct
  (params (Width :type Integer) (Height :type Integer))
  (Variables|Default|SetWidth Width)
  (Variables|Default|SetHeight Height)
  (for _index (range 0 (- (Variables|Default|GetHeight) 1))
    (Variables|Default|SetCurrentZ (* _index 2.5e+02))
    (if (Variables|Default|GetIsDestroyed)
      (for _index_2 (range 0 (- (- (Variables|Default|GetWidth) 1) _index))
        (Variables|Default|SetCurrentX (* _index_2 2.5e+02))
        (if (== (Variables|Default|GetCurrentZ) 0.0)
          (if (== (Variables|Default|GetCurrentX) (* (- (- (Variables|Default|GetWidth) 1) _index) 2.5e+02))
            (AddComponent|AddChildActorComponent false (Math|Transform|MakeTransform (Math|Vector|MakeVector (Variables|Default|GetCurrentX) 0.0 (Variables|Default|GetCurrentZ))))
            (else
              (AddComponent|AddChildActorComponent false (Math|Transform|MakeTransform (Math|Vector|MakeVector (Variables|Default|GetCurrentX) 0.0 (Variables|Default|GetCurrentZ))))))
          (elif (== (Variables|Default|GetCurrentX) (* (- (- (Variables|Default|GetWidth) 1) _index) 2.5e+02))
            (AddComponent|AddChildActorComponent false (Math|Transform|MakeTransform (Math|Vector|MakeVector (Variables|Default|GetCurrentX) 0.0 (Variables|Default|GetCurrentZ))))
            (else
              (AddComponent|AddChildActorComponent false (Math|Transform|MakeTransform (Math|Vector|MakeVector (Variables|Default|GetCurrentX) 0.0 (Variables|Default|GetCurrentZ))))))))
      (else
        (for _index_3 (range 0 (Variables|Default|GetWidth))
          (Variables|Default|SetCurrentX (* _index_3 2.5e+02))
          (if (== (Variables|Default|GetCurrentZ) 0.0)
            (AddComponent|AddChildActorComponent false (Math|Transform|MakeTransform (Math|Vector|MakeVector (Variables|Default|GetCurrentX) 0.0 (Variables|Default|GetCurrentZ))))
            (else
              (AddComponent|AddChildActorComponent false (Math|Transform|MakeTransform (Math|Vector|MakeVector (Variables|Default|GetCurrentX) 0.0 (Variables|Default|GetCurrentZ)))))))))))