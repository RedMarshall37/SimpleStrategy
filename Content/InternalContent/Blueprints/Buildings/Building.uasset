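; Procedural building actor that assembles a randomly sized, stepped facade from modular child actors in its Construction Script.
; Random width, height and depth within set limits drive a 250-unit grid along two perpendicular sides, each floor one module shorter.
; Branches separate ground from upper floors and end from middle pieces, with side pieces rotated and mirrored.
; The depth loop nests inside the width loop, repeating side pieces, and an older loop remains unconnected.
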(fn ConstructionScript
  (LocalVariables|SetCurrentWidth (Math|Random|RandomIntegerinRange 2 (Variables|Default|GetWidth)))
  (LocalVariables|SetCurrentHeight (Math|Random|RandomIntegerinRange 1 (Variables|Default|GetHeight)))
  (LocalVariables|SetCurrentDeep (Math|Random|RandomIntegerinRange 2 (Variables|Default|GetDeep)))
  (for _index (range 0 (LocalVariables|GetCurrentHeight))
    (LocalVariables|SetCurrentZ (* _index 2.5e+02))
    (bind _output_get (LocalVariables|SetCurrentHeightIndex _index))
    (for _index_2 (range 0 (- (LocalVariables|GetCurrentWidth) _output_get))
      (LocalVariables|SetCurrentX (* _index_2 2.5e+02))
      (LocalVariables|SetCurrentWidthtIndex _index_2)
      (if (== (LocalVariables|GetCurrentHeightIndex) 0)
        (if (== (LocalVariables|GetCurrentWidthtIndex) (- (LocalVariables|GetCurrentWidth) _output_get))
          (AddComponent|AddChildActorComponent false (Math|Transform|MakeTransform (Math|Vector|MakeVector (LocalVariables|GetCurrentX) 0.0 (LocalVariables|GetCurrentZ))))
          (else
            (AddComponent|AddChildActorComponent false (Math|Transform|MakeTransform (Math|Vector|MakeVector (LocalVariables|GetCurrentX) 0.0 (LocalVariables|GetCurrentZ))))))
        (elif (== (LocalVariables|GetCurrentWidthtIndex) (- (LocalVariables|GetCurrentWidth) _output_get))
          (AddComponent|AddChildActorComponent false (Math|Transform|MakeTransform (Math|Vector|MakeVector (LocalVariables|GetCurrentX) 0.0 (LocalVariables|GetCurrentZ))))
          (else
            (AddComponent|AddChildActorComponent false (Math|Transform|MakeTransform (Math|Vector|MakeVector (LocalVariables|GetCurrentX) 0.0 (LocalVariables|GetCurrentZ)))))))
      (for _index_3 (range 0 (- (LocalVariables|GetCurrentDeep) (LocalVariables|GetCurrentHeightIndex)))
        (LocalVariables|SetCurrentY (* _index_3 2.5e+02))
        (LocalVariables|SetCurrentDeepIndex _index_3)
        (if (== (LocalVariables|GetCurrentHeightIndex) 0)
          (if (== (LocalVariables|GetCurrentDeepIndex) (- (LocalVariables|GetCurrentDeep) (LocalVariables|GetCurrentHeightIndex)))
            (AddComponent|AddChildActorComponent false (Math|Transform|MakeTransform (Math|Vector|MakeVector 0.0 (LocalVariables|GetCurrentY) (LocalVariables|GetCurrentZ)) "0,-90.000000, 0" "-1.000000,1,1"))
            (else
              (AddComponent|AddChildActorComponent false (Math|Transform|MakeTransform (Math|Vector|MakeVector 0.0 (LocalVariables|GetCurrentY) (LocalVariables|GetCurrentZ)) "0,-90.000000, 0" "-1.000000,1,1"))))
          (elif (== (LocalVariables|GetCurrentDeepIndex) (- (LocalVariables|GetCurrentDeep) (LocalVariables|GetCurrentHeightIndex)))
            (AddComponent|AddChildActorComponent false (Math|Transform|MakeTransform (Math|Vector|MakeVector 0.0 (LocalVariables|GetCurrentY) (LocalVariables|GetCurrentZ)) "0,-90.000000, 0" "-1.000000,1,1"))
            (else
              (AddComponent|AddChildActorComponent false (Math|Transform|MakeTransform (Math|Vector|MakeVector 0.0 (LocalVariables|GetCurrentY) (LocalVariables|GetCurrentZ)) "0,-90.000000, 0" "-1.000000,1,1")))))))))