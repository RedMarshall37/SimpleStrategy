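; Squad generator Blueprint that spawns a linked command hierarchy of units at given coordinates.
; SpawnSquare creates a Sergeant and an Officer at the same point, registers the Officer with the Sergeant and sets the back-reference.
; It then spawns a row of seven UnitBase actors evenly spaced along +Y from that point, each pointing to the Officer as its superior.
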(fn ConstructionScript)

(fn SpawnSquare
  (params (Coordinates :type Vector))
  (LocalVariables|SetLocalCoordinates Coordinates)
  (bind _returnvalue (Game|SpawnActorfromClass "/Game/InternalContent/Blueprints/Units/Sergeant.Sergeant_C" (Math|Transform|MakeTransform Coordinates) "Undefined" 0 0))
  (LocalVariables|SetSergeant _returnvalue)
  (bind _returnvalue_2 (Game|SpawnActorfromClass "/Game/InternalContent/Blueprints/Units/Officer.Officer_C" (Math|Transform|MakeTransform (LocalVariables|GetLocalCoordinates)) "Undefined" 0 0))
  (bind _output_get (LocalVariables|SetOfficer _returnvalue_2))
  (Utilities|Array|Add (Variables|/Game/InternalContent/Blueprints/Units/Sergeant.Sergeant_C|GetOfficers (LocalVariables|GetSergeant)) _output_get)
  (Variables|/Game/InternalContent/Blueprints/Units/Officer.Officer_C|SetSergeant (LocalVariables|GetOfficer) (LocalVariables|GetSergeant))
  (for _index (range 1 7)
    (bind _returnvalue_3 (Game|SpawnActorfromClass "/Game/InternalContent/Blueprints/Units/UnitBase.UnitBase_C" (Math|Transform|MakeTransform (Math|Vector|MakeVector (.x (LocalVariables|GetLocalCoordinates)) (+ (.y (LocalVariables|GetLocalCoordinates)) (* _index 1.5e+02)) (.z (LocalVariables|GetLocalCoordinates)))) "Undefined" 0 0))
    (Variables|/Game/InternalContent/Blueprints/Units/UnitBase.UnitBase_C|SetOfficer _returnvalue_3 (LocalVariables|GetOfficer))))