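; TwoPointPipe is a construction-script Blueprint that stretches a Cylinder component according to two point components, PointStart and PointEnd.
; It sets the cylinder's relative rotation from the look-at rotation between their world locations, adding 90 degrees of pitch to align its Z axis.
; World Z scale is the distance divided by 100, keeping X and Y.
; World location is the sum of both points, without halving to a midpoint.
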(fn ConstructionScript
  (bind _cylinder (Variables|Default|GetCylinder))
  (bind _returnvalue (Transformation|GetWorldTransform _cylinder))
  (LocalVariables|SetStartPointLocation (Transformation|GetWorldLocation (Variables|Default|GetPointStart)))
  (LocalVariables|SetEndPointLocation (Transformation|GetWorldLocation (Variables|Components|GetPointEnd)))
  (Transformation|SetRelativeRotation (Variables|Default|GetCylinder) (Math|Rotator|MakeRotator (.roll (Math|Rotator|FindLookatRotation (LocalVariables|GetStartPointLocation) (LocalVariables|GetEndPointLocation))) (+ (.pitch (Math|Rotator|FindLookatRotation (LocalVariables|GetStartPointLocation) (LocalVariables|GetEndPointLocation))) 9e+01) (.yaw (Math|Rotator|FindLookatRotation (LocalVariables|GetStartPointLocation) (LocalVariables|GetEndPointLocation)))) false false)
  (Transformation|SetWorldLocation (Variables|Default|GetCylinder) (Math|Vector|MakeVector (.x (+ (LocalVariables|GetStartPointLocation) (LocalVariables|GetEndPointLocation))) (.y (+ (LocalVariables|GetStartPointLocation) (LocalVariables|GetEndPointLocation))) (.z (+ (LocalVariables|GetStartPointLocation) (LocalVariables|GetEndPointLocation)))) false false)
  (Transformation|SetWorldScale3D (Variables|Default|GetCylinder) (Math|Vector|MakeVector (.x (.scale _returnvalue)) (.y (.scale _returnvalue)) (/ (Math|Vector|Distance(Vector) (LocalVariables|GetStartPointLocation) (LocalVariables|GetEndPointLocation)) 1e+02))))