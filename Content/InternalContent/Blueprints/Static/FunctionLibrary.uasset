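; Static function library with helpers for ranking actors by distance and choosing places for units.
; FindNearestActor selection-sorts an actor array in place by distance to a primary unit and returns the whole array.
; CheckPlace rejects occupied places and accepts any free one if the unit has none.
; Otherwise the place must differ from the current one, face the target within tolerance and, when approaching, be closer to it.
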(fn FindNearestActor
  (params (AllActors :type Array%20of%20Actor%20Object%20References) (PrimaryUnit :type Actor%20Object%20Reference))
  (bind _output_get (LocalVariables|SetAll%20Actors AllActors))
  (for (_ _array_index) _output_get
    (bind _output_get_2 (LocalVariables|SetCurrentIndexOffset _array_index))
    (bind _output_get_3 (LocalVariables|SetIndexElementWithMinDistance _output_get_2))
    (for _index (range _output_get_3 (- (Utilities|Array|Length (LocalVariables|GetAll%20Actors)) 1))
      (if (< (Transformation|GetDistanceTo (Utilities|Array|Get(acopy) (LocalVariables|GetAll%20Actors) _index) PrimaryUnit) (Transformation|GetDistanceTo (Utilities|Array|Get(acopy) (LocalVariables|GetAll%20Actors) (LocalVariables|GetIndexElementWithMinDistance)) PrimaryUnit))
        (LocalVariables|SetIndexElementWithMinDistance _index)))
    (Utilities|Array|Swap (LocalVariables|GetAll%20Actors) (LocalVariables|GetIndexElementWithMinDistance) (LocalVariables|GetCurrentIndexOffset)))
  (return (LocalVariables|GetAll%20Actors)))

(fn CheckPlace
  (params (PlaceModel :type Scene%20Component%20Object%20Reference) (Place :type Place%20Object%20Reference) (Unit :type Unit%20Base%20Object%20Reference) (TargetCoordinates :type Vector%20%28by%20ref%29) (Approach :type Boolean))
  (LocalVariables|SetPlace%20Model PlaceModel)
  (LocalVariables|SetAs%20Place Place)
  (LocalVariables|SetAs%20Unit Unit)
  (LocalVariables|SetTarget%20Coordinates TargetCoordinates)
  (LocalVariables|SetCurrent%20Approach Approach)
  (if (Utilities|IsValid (.attachedunit (Variables|/Game/InternalContent/Blueprints/Places/Place.Place_C|GetPlaceStruct (LocalVariables|GetAs%20Place))))
    (return false)
    (else
      (Utilities|IsValid (Variables|/Game/InternalContent/Blueprints/Units/UnitBase.UnitBase_C|GetCurrentPlace (LocalVariables|GetAs%20Unit))
        (:Is%20Valid
          (if (and (Math|Rotator|Equal(Rotator) (Math|Rotator|FindLookatRotation (Transformation|GetActorLocation (LocalVariables|GetAs%20Place)) (LocalVariables|GetTarget%20Coordinates)) (Math|Rotator|MakeRotator (.roll (Transformation|GetWorldRotation (LocalVariables|GetPlace%20Model))) (.pitch (Transformation|GetWorldRotation (LocalVariables|GetPlace%20Model))) (+ (.yaw (Transformation|GetWorldRotation (LocalVariables|GetPlace%20Model))) 9e+01)) 9e+01) (Math|Vector|NotEqual(Vector) (Transformation|GetActorLocation (LocalVariables|GetAs%20Place)) (Transformation|GetActorLocation (Variables|/Game/InternalContent/Blueprints/Units/UnitBase.UnitBase_C|GetCurrentPlace (LocalVariables|GetAs%20Unit))) 1e+01))
            (if (LocalVariables|GetCurrent%20Approach)
              (if (> (Math|Vector|Distance(Vector) (Transformation|GetActorLocation (Variables|/Game/InternalContent/Blueprints/Units/UnitBase.UnitBase_C|GetCurrentPlace (LocalVariables|GetAs%20Unit))) (LocalVariables|GetTarget%20Coordinates)) (Math|Vector|Distance(Vector) (Transformation|GetActorLocation (LocalVariables|GetAs%20Place)) (LocalVariables|GetTarget%20Coordinates)))
                _
                (else
                  (return false))))
            (return true)
            (else
              (return false))))
        (:Is%20Not%20Valid
          (return true))))))