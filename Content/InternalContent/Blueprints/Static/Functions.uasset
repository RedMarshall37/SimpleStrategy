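; Actor Blueprint in a Static folder that holds a utility function, FindNearestActor, with its event graph and construction script left empty.
; The function gathers all actors of a given class and orders them by distance to a primary unit using an in-place selection sort.
; Despite its name, it returns the whole array, nearest first, rather than a single actor.
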(event EventBeginPlay)

(event Collision|EventActorBeginOverlap
  (params (OtherActor :type Actor%20Object%20Reference)))

(event EventTick
  (params (DeltaSeconds :type Float%20%28single-precision%29)))

(fn ConstructionScript)

(fn FindNearestActor
  (params (ActorClass :type Actor%20Class%20Reference) (PrimaryUnit :type Actor%20Object%20Reference))
  (bind _outactors (Actor|GetAllActorsOfClass ActorClass))
  (bind _output_get (LocalVariables|SetAllActors _outactors))
  (for (_ _array_index) _output_get
    (bind _output_get_2 (LocalVariables|SetCurrentIndexOffset _array_index))
    (bind _output_get_3 (LocalVariables|SetIndexElementWithMinDistance _output_get_2))
    (for _index (range _output_get_3 (- (Utilities|Array|Length (LocalVariables|GetAllActors)) 1))
      (if (< (Transformation|GetDistanceTo (Utilities|Array|Get(acopy) (LocalVariables|GetAllActors) _index) PrimaryUnit) (Transformation|GetDistanceTo (Utilities|Array|Get(acopy) (LocalVariables|GetAllActors) (LocalVariables|GetIndexElementWithMinDistance)) PrimaryUnit))
        (LocalVariables|SetIndexElementWithMinDistance _index)))
    (Utilities|Array|Swap (LocalVariables|GetAllActors) (LocalVariables|GetIndexElementWithMinDistance) (LocalVariables|GetCurrentIndexOffset)))
  (return (LocalVariables|GetAllActors)))